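; BP_Racer_Pawn_AI is a racer pawn, named as the AI variant, with its player-control logic disconnected.
; On Hit it forwards the colliding actor, component and location to BPDamageableActor to apply collision damage.
; The construction script registers thruster particle systems with BPVisualEffects and caches BPEntity.
; Input, BeginPlay and Tick events are empty; flight, drift, ramming, marker-scan and beacon-spawn chains remain but never run.
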(event `EnhancedInput|/Game/Input/IA_Number_5`
  (params (ActionValue :type Boolean) (ElapsedSeconds :type "Float (double-precision)") (TriggeredSeconds :type "Float (double-precision)") (InputAction :type "InputAction Object Reference" :default "/Game/Input/IA_Number_5.IA_Number_5")))

(event `EnhancedInput|/Game/Input/IA_Number_4`
  (params (ActionValue :type Boolean) (ElapsedSeconds :type "Float (double-precision)") (TriggeredSeconds :type "Float (double-precision)") (InputAction :type "InputAction Object Reference" :default "/Game/Input/IA_Number_4.IA_Number_4")))

(event `EnhancedInput|/Game/Input/IA_Number_3`
  (params (ActionValue :type Boolean) (ElapsedSeconds :type "Float (double-precision)") (TriggeredSeconds :type "Float (double-precision)") (InputAction :type "InputAction Object Reference" :default "/Game/Input/IA_Number_3.IA_Number_3")))

(event `self.ReceiveBeginPlay`)

(event `EnhancedInput|/Game/Input/IA_Look`
  (params (ActionValue :type "Vector2D Structure") (ElapsedSeconds :type "Float (double-precision)") (TriggeredSeconds :type "Float (double-precision)") (InputAction :type "InputAction Object Reference" :default "/Game/Input/IA_Look.IA_Look")))

(event `EnhancedInput|/Game/Input/IA_Button_F`
  (params (ActionValue :type Boolean) (ElapsedSeconds :type "Float (double-precision)") (TriggeredSeconds :type "Float (double-precision)") (InputAction :type "InputAction Object Reference" :default "/Game/Input/IA_Button_F.IA_Button_F")))

(event `self.ReceiveTick`
  (params (DeltaSeconds :type "Float (single-precision)")))

(event `EnhancedInput|/Game/Input/IA_Right_Click`
  (params (ActionValue :type Boolean) (ElapsedSeconds :type "Float (double-precision)") (TriggeredSeconds :type "Float (double-precision)") (InputAction :type "InputAction Object Reference" :default "/Game/Input/IA_Right_Click.IA_Right_Click")))

(event `EnhancedInput|/Game/Input/IA_Fly_Up`
  (params (ActionValue :type Boolean) (ElapsedSeconds :type "Float (double-precision)") (TriggeredSeconds :type "Float (double-precision)") (InputAction :type "InputAction Object Reference" :default "/Game/Input/IA_Fly_Up.IA_Fly_Up")))

(event `EnhancedInput|/Game/Input/IA_Fly_Left`
  (params (ActionValue :type Boolean) (ElapsedSeconds :type "Float (double-precision)") (TriggeredSeconds :type "Float (double-precision)") (InputAction :type "InputAction Object Reference" :default "/Game/Input/IA_Fly_Left.IA_Fly_Left")))

(event `EnhancedInput|/Game/Input/IA_Fly_Down`
  (params (ActionValue :type Boolean) (ElapsedSeconds :type "Float (double-precision)") (TriggeredSeconds :type "Float (double-precision)") (InputAction :type "InputAction Object Reference" :default "/Game/Input/IA_Fly_Down.IA_Fly_Down")))

(event `self.ReceiveHit`
  (params (MyComp :type "PrimitiveComponent Object Reference") (Other :type "Actor Object Reference") (OtherComp :type "PrimitiveComponent Object Reference") (bSelfMoved :type Boolean) (HitLocation :type "Vector Structure") (HitNormal :type "Vector Structure") (NormalImpulse :type "Vector Structure") (Hit :type "HitResult Structure (by ref)"))
  (`/Game/Blueprints/BlueprintComponents/BP_DamageableActor.ApplyDamageFromCollision` (`self.BP_DamageableActor`) Other OtherComp HitLocation))

(event `EnhancedInput|/Game/Input/IA_Fly_Right`
  (params (ActionValue :type Boolean) (ElapsedSeconds :type "Float (double-precision)") (TriggeredSeconds :type "Float (double-precision)") (InputAction :type "InputAction Object Reference" :default "/Game/Input/IA_Fly_Right.IA_Fly_Right")))

(fn `UserConstructionScript`
  (bind _thrusters (`Class_VisualEffects.thrusters` (`self.BP_VisualEffects`)))
  (`KismetArrayLibrary.Array_Add` _thrusters (`self.ParticleSystem`))
  (`KismetArrayLibrary.Array_Add` _thrusters (`self.ParticleSystem1`))
  (`KismetArrayLibrary.Array_Add` _thrusters (`self.ParticleSystemArmR`))
  (`KismetArrayLibrary.Array_Add` _thrusters (`self.ParticleSystemArmL`))
  (set `self.entityPtr` (`self.BP_Entity`)))