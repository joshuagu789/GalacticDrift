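; BP_Police is a police escort that stores its orbit component's target racer as the caller and attacks enemies entering its overlap area.
; An entity component check flags enemies, which join a target list, draw the swivel's facing, and get cannon fire after a delay.
; Overlap end removes targets.
; Tick cycles to the next target when none is active, attacking immediately, or faces the calling racer if none remain.
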(event `self.ReceiveBeginPlay`
  (`KismetSystemLibrary.Delay` 0.1)
  (bind _returnvalue (`Class_OrbitMovement.GetOrbitTarget` (`self.BP_OrbitMovement`)))
  (bind _asclass_racer_pawn (cast `Class_Racer_Pawn` _returnvalue))
  (set `self.callingRacer` _asclass_racer_pawn))

(event `self.ReceiveActorBeginOverlap`
  (params (OtherActor :type "Actor Object Reference"))
  (bind _returnvalue (`self.GetComponentByClass` OtherActor "/Game/Blueprints/BlueprintComponents/BP_Entity.BP_Entity_C"))
  (bind _target (`self.target`))
  (if (`KismetSystemLibrary.IsValid` _returnvalue)
    (bind _returnvalue_2 (`Class_Entity.IsEnemyWith` (`self.BP_Entity`) (`Class_Entity.type` _returnvalue)))
    (if _returnvalue_2
      (`self.AddTarget` OtherActor)
      (`Class_Swivel.BeginFacing` (`self.BP_Swivel`) _target)
      (`KismetSystemLibrary.Delay` 4.5)
      (`Class_Cannon.BeginAttacking` (`self.BP_Cannon`) _target)
      (`KismetSystemLibrary.PrintString` (`KismetStringLibrary.Concat_StrStr` "Police Attacking: " (`KismetSystemLibrary.GetDisplayName` _target))))))

(event `self.ReceiveActorEndOverlap`
  (params (OtherActor :type "Actor Object Reference"))
  (bind _returnvalue (`self.HasActorInTargetList` OtherActor))
  (if _returnvalue
    (`self.RemoveTarget` OtherActor)))

(event `self.ReceiveTick`
  (params (DeltaSeconds :type "Float (single-precision)"))
  (bind _target (`self.target`))
  (bind _callingracer (`self.callingRacer`))
  (bind _returnvalue (`self.HasTarget`))
  (if (not _returnvalue)
    (bind _returnvalue_2 (`self.CycleNextTarget`))
    (if _returnvalue_2
      (`Class_Swivel.BeginFacing` (`self.BP_Swivel`) _target)
      (`Class_Cannon.BeginAttacking` (`self.BP_Cannon`) _target)
      (elif (`KismetSystemLibrary.IsValid` _callingracer)
        (`Class_Swivel.BeginFacing` (`self.BP_Swivel`) _callingracer)))))

(fn `UserConstructionScript`
  (set `Class_OrbitMovement.moveComponentPtr` (`self.FloatingPawnMovement`) (`self.BP_OrbitMovement`)))