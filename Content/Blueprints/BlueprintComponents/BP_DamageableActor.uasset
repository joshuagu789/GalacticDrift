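; Damageable component that applies collision damage to its owning actor and handles destruction by type.
; Once destroyed, geometry collections crumble for a limited number of hits, ragdollable actors ragdoll and reset health, and explodable actors self-destruct.
; Self-destruct spawns the destroyed-version class, crumbles it if its root is a geometry collection, and destroys the owner.
; Crumbled pieces receive a radial impulse from the hit point, scaled by squared mass and a force factor.
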(event `self.ReceiveBeginPlay`)

(event `self.ReceiveTick`
  (params (DeltaSeconds :type "Float (single-precision)")))

(fn `ApplyDamageFromCollision`
  (params (collisionSourceActor :type "Actor Object Reference") (collisionSourcePrimitiveComponent :type "PrimitiveComponent Object Reference") (hitLocation :type "Vector Structure"))
  (bind _returnvalue (`Actor.GetComponentByClass` (`self.GetOwner`) "/Script/GeometryCollectionEngine.GeometryCollectionComponent"))
  (`self.CalculateAndApplyDamage` collisionSourcePrimitiveComponent)
  (bind _returnvalue_2 (`self.GetType`))
  (switch `DamageableActor_Type` _returnvalue_2
    (:`GEOMETRY_COLLECTION`
      (if (> (`self.numCollisions`) 0)
        (bind _returnvalue_3 (`self.IsDestroyed`))
        (if _returnvalue_3
          (if (`KismetSystemLibrary.IsValid` _returnvalue)
            (`GeometryCollectionComponent.CrumbleActiveClusters` _returnvalue)
            (`self.ApplyForceOnCrumbledGeometryCollection` _returnvalue (`local.hitLocation`))
            (set `self.numCollisions` (- (`self.numCollisions`) 1))))))
    (:`EXPLODABLE`
      (bind _returnvalue_4 (`self.IsDestroyed`))
      (if _returnvalue_4
        (`self.SelfDestruct` (`local.hitLocation`))))
    (:`RAGDOLLABLE`
      (bind _returnvalue_5 (`self.IsDestroyed`))
      (if _returnvalue_5
        (`self.Ragdoll`)
        (`self.ResetHealth`)))))

(fn `ApplyForceOnCrumbledGeometryCollection`
  (params (geometryCollection :type "GeometryCollectionComponent Object Reference") (explosionLocation :type "Vector Structure"))
  (bind _returnvalue (`PrimitiveComponent.GetMass` geometryCollection))
  (`PrimitiveComponent.AddRadialImpulse` geometryCollection explosionLocation (`KismetMathLibrary.VSize` (- explosionLocation (`PrimitiveComponent.GetCenterOfMass` geometryCollection "None"))) (* (* _returnvalue _returnvalue) (`self.explosionForceFactor`)) "RIF_Constant" false))

(fn `SelfDestruct`
  (params (explosionLocation :type "Vector Structure"))
  (bind _destroyedversionptr (`self.destroyedVersionPtr`))
  (if (`KismetSystemLibrary.IsValidClass` _destroyedversionptr)
    (bind _returnvalue (`|SpawnActorFromClass` _destroyedversionptr (`Actor.GetTransform` (`self.GetOwner`)) "AlwaysSpawn" "MultiplyWithRoot" null null))
    (bind _asgeometry_collection_component (cast `GeometryCollectionComponent` (`Actor.RootComponent` _returnvalue))
      (:`then`
        (`GeometryCollectionComponent.CrumbleActiveClusters` _asgeometry_collection_component)
        (`self.ApplyForceOnCrumbledGeometryCollection` _asgeometry_collection_component (`local.explosionLocation`)))
      (:`CastFailed`
        _))
    (`Actor.K2_DestroyActor` (`self.GetOwner`))))