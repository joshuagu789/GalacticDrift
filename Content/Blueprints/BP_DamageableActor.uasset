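; Damage handler that applies collision damage and swaps its owning actor for a fractured version when an explodable is destroyed.
; ApplyDamageFromCollision calculates and applies damage, prints the result, then checks the type and destroyed state.
; For destroyed explodables, it spawns the DestroyedVersionPtr class at the owner's transform, crumbles its Geometry Collection root and destroys the owner.
; An unconnected BP_FracturedBody spawn path with manual physics setup never runs.
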(fn `ApplyDamageFromCollision`
  (bind _destroyedversionptr (`self.destroyedVersionPtr`))
  (bind _returnvalue (`self.CalculateAndApplyDamage`))
  (`KismetSystemLibrary.PrintString` (`KismetStringLibrary.Conv_DoubleToString` _returnvalue))
  (bind _returnvalue_2 (`self.GetType`))
  (switch `DamageableActor_Type` _returnvalue_2
    (:`EXPLODABLE`
      (bind _returnvalue_3 (`self.IsDestroyed`))
      (if _returnvalue_3
        (if (`KismetSystemLibrary.IsValidClass` _destroyedversionptr)
          (bind _returnvalue_4 (`|SpawnActorFromClass` _destroyedversionptr (`Actor.GetTransform` (`self.GetOwner`)) "AlwaysSpawn" "MultiplyWithRoot" null null))
          (bind _asgeometry_collection_component (cast `GeometryCollectionComponent` (`Actor.RootComponent` _returnvalue_4)))
          (`GeometryCollectionComponent.CrumbleActiveClusters` _asgeometry_collection_component)
          (`Actor.K2_DestroyActor` (`self.GetOwner`)))))))