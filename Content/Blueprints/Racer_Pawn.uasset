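; Player-controlled racer pawn that flies with auto-acceleration and drifts in four directions, marking itself as a racer.
; BeginPlay adds the Enhanced Input context and hands its floating movement component and skeletal mesh to flight functions defined outside these graphs.
; Look input steers the controller, while fly inputs drive drifting until released.
; Tick sends speed to the HUD, and hits trigger a timed ragdoll and recovery.
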(event `self.ReceiveBeginPlay`
  (`Class_Marker.SetType` (`self.Class_Marker`) "RACER")
  (bind _asplayer_controller (cast `PlayerController` (`self.GetController`)))
  (bind _returnvalue (pcsubsystem `EnhancedInputLocalPlayerSubsystem` _asplayer_controller))
  (`/Engine/EditorBlueprintResources/StandardMacros.IsValid` _returnvalue
    (:`Is Valid`
      (`EnhancedInputSubsystemInterface.AddMappingContext` _returnvalue "/Game/Input/IMC_Racer.IMC_Racer" 0 (struct))
      (set `self.moveComponentPtr` (`self.FloatingPawnMovement`))
      (set `self.skeletalMeshPtr` (`self.Mesh`))
      (`self.StartFlying` 0.7 true 0.1))))

(event `EnhancedInput|/Game/Input/IA_Look`
  (params (ActionValue :type "Vector2D Structure") (ElapsedSeconds :type "Float (double-precision)") (TriggeredSeconds :type "Float (double-precision)") (InputAction :type "InputAction Object Reference" :default "/Game/Input/IA_Look.IA_Look"))
  (:`Triggered`
    (`self.AddControllerYawInput` ActionValue_X)
    (`self.AddControllerPitchInput` (* -1.0 ActionValue_Y))))

(event `self.ReceiveTick`
  (params (DeltaSeconds :type "Float (single-precision)"))
  (bind _asbp_in_game_hud (cast `/Game/Blueprints/BP_InGameHUD` (`PlayerController.GetHUD` (`GameplayStatics.GetPlayerController` 0))))
  (bind _returnvalue (`Class_ActorInformationTracker.GetSpeedIntAsString`))
  (`/Game/UI/BP_InGameWidget.UpdateSpeed` (`/Game/Blueprints/BP_InGameHUD.UI Ref` _asbp_in_game_hud) _returnvalue))

(event `EnhancedInput|/Game/Input/IA_Fly_Up`
  (params (ActionValue :type Boolean) (ElapsedSeconds :type "Float (double-precision)") (TriggeredSeconds :type "Float (double-precision)") (InputAction :type "InputAction Object Reference" :default "/Game/Input/IA_Fly_Up.IA_Fly_Up"))
  (:`Triggered`
    (`self.CanDrift` :!label _label)
    (`self.DriftUp` 4.0))
  (:`Ongoing`
    (goto _label))
  (:`Completed`
    (`self.StopDrift` :!label _label_2)))

(event `EnhancedInput|/Game/Input/IA_Fly_Left`
  (params (ActionValue :type Boolean) (ElapsedSeconds :type "Float (double-precision)") (TriggeredSeconds :type "Float (double-precision)") (InputAction :type "InputAction Object Reference" :default "/Game/Input/IA_Fly_Left.IA_Fly_Left"))
  (:`Triggered`
    (`self.CanDrift` :!label _label_3)
    (`self.DriftLeft` 4.0))
  (:`Ongoing`
    (goto _label_3))
  (:`Completed`
    (goto _label_2)))

(event `self.ReceiveHit`
  (params (MyComp :type "PrimitiveComponent Object Reference") (Other :type "Actor Object Reference") (OtherComp :type "PrimitiveComponent Object Reference") (bSelfMoved :type Boolean) (HitLocation :type "Vector Structure") (HitNormal :type "Vector Structure") (NormalImpulse :type "Vector Structure") (Hit :type "HitResult Structure (by ref)"))
  (`Ragdollable.RagdollFor` 5.0)
  (`KismetSystemLibrary.Delay` 4.0)
  (`Ragdollable.UnRagdoll`))

(event `EnhancedInput|/Game/Input/IA_Fly_Down`
  (params (ActionValue :type Boolean) (ElapsedSeconds :type "Float (double-precision)") (TriggeredSeconds :type "Float (double-precision)") (InputAction :type "InputAction Object Reference" :default "/Game/Input/IA_Fly_Down.IA_Fly_Down"))
  (:`Triggered`
    (`self.CanDrift` :!label _label_4)
    (`self.DriftDown` 4.0))
  (:`Ongoing`
    (goto _label_4))
  (:`Completed`
    (goto _label_2)))

(event `EnhancedInput|/Game/Input/IA_Fly_Right`
  (params (ActionValue :type Boolean) (ElapsedSeconds :type "Float (double-precision)") (TriggeredSeconds :type "Float (double-precision)") (InputAction :type "InputAction Object Reference" :default "/Game/Input/IA_Fly_Right.IA_Fly_Right"))
  (:`Triggered`
    (`self.CanDrift` :!label _label_5)
    (`self.DriftRight` 4.0))
  (:`Ongoing`
    (goto _label_5))
  (:`Completed`
    (goto _label_2)))

(fn `UserConstructionScript`)