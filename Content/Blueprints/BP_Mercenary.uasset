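; BP_Mercenary is an AI combatant that orbits, faces and fires on the closest enemy.
; While it lacks a target, Tick requests the closest one from the server, then hands it to the BPSwivel, BPOrbitMovement and BPCannon components.
; Orbit movement drives the FloatingPawnMovement, and collision hits feed BPDamageableActor, which is linked to BPEntity at construction.
; Delayed ragdoll physics and server-removal logic exist but are unconnected.
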(event `self.ReceiveBeginPlay`
  (set `Class_OrbitMovement.moveComponentPtr` (`self.FloatingPawnMovement`) (`self.BP_OrbitMovement`)))

(event `self.ReceiveHit`
  (params (MyComp :type "PrimitiveComponent Object Reference") (Other :type "Actor Object Reference") (OtherComp :type "PrimitiveComponent Object Reference") (bSelfMoved :type Boolean) (HitLocation :type "Vector Structure") (HitNormal :type "Vector Structure") (NormalImpulse :type "Vector Structure") (Hit :type "HitResult Structure (by ref)"))
  (`/Game/Blueprints/BlueprintComponents/BP_DamageableActor.ApplyDamageFromCollision` (`self.BP_DamageableActor`) Other OtherComp HitLocation))

(event `self.ReceiveDestroyed`)

(event `self.ReceiveTick`
  (params (DeltaSeconds :type "Float (single-precision)"))
  (bind _target (`self.target`))
  (bind _returnvalue (`self.HasTarget`))
  (if (not _returnvalue)
    (`/Game/Blueprints/BP_FunctionLibrary.TargetClosestEnemyFromServer` (`self.BP_Entity`) self)
    (bind _returnvalue_2 (`self.HasTarget`))
    (if _returnvalue_2
      (`Class_Swivel.BeginFacing` (`self.BP_Swivel`) _target)
      (`Class_OrbitMovement.BeginOrbiting` (`self.BP_OrbitMovement`) _target)
      (`Class_Cannon.BeginAttacking` (`self.BP_Cannon`) _target))))

(fn `UserConstructionScript`
  (set `Class_DamageableActor.entityPtr` (`self.BP_Entity`) (`self.BP_DamageableActor`)))