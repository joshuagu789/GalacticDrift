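; BP_PlayerUI feeds a racer pawn's speed to the in-game HUD, and appears to be a component on that pawn.
; On BeginPlay it caches the first player's BP_InGameHUD and its UI widget reference.
; Every tick it casts its owner to Class_Racer_Pawn and passes the speed string to the widget.
; UpdateMarkers is an empty stub.
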(event `self.ReceiveBeginPlay`
  (bind _asbp_in_game_hud (cast `/Game/Blueprints/BP_InGameHUD` (`PlayerController.GetHUD` (`GameplayStatics.GetPlayerController` 0))))
  (set `self.HUD_Ptr` _asbp_in_game_hud)
  (set `self.widget_Ptr` (`/Game/Blueprints/BP_InGameHUD.UI Ref` _asbp_in_game_hud)))

(event `self.ReceiveTick`
  (params (DeltaSeconds :type "Float (single-precision)"))
  (`self.UpdateSpeed`))

(fn `UpdateMarkers`
  (params (NewParam :type Boolean)))

(fn `UpdateSpeed`
  (bind _asclass_racer_pawn (cast `Class_Racer_Pawn` (`self.GetOwner`)))
  (bind _returnvalue (`Class_ActorInformationTracker.GetSpeedIntAsString` _asclass_racer_pawn))
  (`/Game/UI/BP_InGameWidget.UpdateSpeed` (`self.widget_Ptr`) _returnvalue))