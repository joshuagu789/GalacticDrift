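; Player-controlled flying racer pawn that constantly thrusts itself forward while the player steers it.
; On BeginPlay it adds the racer Enhanced Input mapping context, and every Tick pushes the capsule along the actor's forward vector.
; Four fly actions apply fixed pitch or yaw world-rotation steps while held, independent of frame time, and look input drives controller rotation.
; Standard movement-input logic remains but is disconnected.
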(event `EnhancedInput|/Game/Input/IA_Look`
  (params (ActionValue :type "Vector2D Structure") (ElapsedSeconds :type "Float (double-precision)") (TriggeredSeconds :type "Float (double-precision)") (InputAction :type "InputAction Object Reference" :default "/Game/Input/IA_Look.IA_Look"))
  (:`Triggered`
    (`self.AddControllerYawInput` ActionValue_X)
    (`self.AddControllerPitchInput` (* -1.0 ActionValue_Y))))

(event `self.ReceiveBeginPlay`
  (bind _asplayer_controller (cast `PlayerController` (`self.GetController`)))
  (bind _returnvalue (pcsubsystem `EnhancedInputLocalPlayerSubsystem` _asplayer_controller))
  (`/Engine/EditorBlueprintResources/StandardMacros.IsValid` _returnvalue
    (:`Is Valid`
      (`EnhancedInputSubsystemInterface.AddMappingContext` _returnvalue "/Game/Input/IMC_Racer.IMC_Racer" 0 (struct)))))

(event `EnhancedInput|/Game/Input/IA_Fly_Tutorial`
  (params (ActionValue :type "Vector2D Structure") (ElapsedSeconds :type "Float (double-precision)") (TriggeredSeconds :type "Float (double-precision)") (InputAction :type "InputAction Object Reference" :default "/Game/Input/IA_Fly_Tutorial.IA_Fly_Tutorial")))

(event `self.ReceiveTick`
  (params (DeltaSeconds :type "Float (single-precision)"))
  (`PrimitiveComponent.AddForce` (`self.CapsuleComponent`) (* (`self.GetActorForwardVector`) 50000.0) "None" false))

(event `EnhancedInput|/Game/Input/IA_Fly_Up`
  (params (ActionValue :type Boolean) (ElapsedSeconds :type "Float (double-precision)") (TriggeredSeconds :type "Float (double-precision)") (InputAction :type "InputAction Object Reference" :default "/Game/Input/IA_Fly_Up.IA_Fly_Up"))
  (:`Triggered`
    (`self.K2_AddActorWorldRotation` (struct :`Pitch` 5.0) true true :!label _label))
  (:`Ongoing`
    (goto _label)))

(event `EnhancedInput|/Game/Input/IA_Fly_Left`
  (params (ActionValue :type Boolean) (ElapsedSeconds :type "Float (double-precision)") (TriggeredSeconds :type "Float (double-precision)") (InputAction :type "InputAction Object Reference" :default "/Game/Input/IA_Fly_Left.IA_Fly_Left"))
  (:`Triggered`
    (`self.K2_AddActorWorldRotation` (struct :`Yaw` -5.0) true true :!label _label_2))
  (:`Ongoing`
    (goto _label_2)))

(event `EnhancedInput|/Game/Input/IA_Fly_Down`
  (params (ActionValue :type Boolean) (ElapsedSeconds :type "Float (double-precision)") (TriggeredSeconds :type "Float (double-precision)") (InputAction :type "InputAction Object Reference" :default "/Game/Input/IA_Fly_Down.IA_Fly_Down"))
  (:`Triggered`
    (`self.K2_AddActorWorldRotation` (struct :`Pitch` -5.0) true true :!label _label_3))
  (:`Ongoing`
    (goto _label_3)))

(event `EnhancedInput|/Game/Input/IA_Fly_Right`
  (params (ActionValue :type Boolean) (ElapsedSeconds :type "Float (double-precision)") (TriggeredSeconds :type "Float (double-precision)") (InputAction :type "InputAction Object Reference" :default "/Game/Input/IA_Fly_Right.IA_Fly_Right"))
  (:`Triggered`
    (`self.K2_AddActorWorldRotation` (struct :`Yaw` 5.0) true true :!label _label_4))
  (:`Ongoing`
    (goto _label_4)))

(fn `UserConstructionScript`)